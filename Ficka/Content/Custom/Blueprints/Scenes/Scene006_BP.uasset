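; Animated beach scene actor with a sun, beach house, boat, fish and dolphin that reveals itself in stages on BeginPlay.
; Construction hides the actor and pauses its "Play"-tagged skeletal meshes, then chained timelines scale in the scene, sun, house and boat.
; Tagged meshes are then unhidden and unpaused in staggered order.
; A fast looping timer rotates fish groups, turns the sun toward the camera and sets the dolphin's Jump by boat proximity.
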(event Custom|MoveFish
  (Transformation|AddRelativeRotation (Variables|Default|GetFishGroup_01) "0,0.050000, 0" false false)
  (Transformation|AddRelativeRotation (Variables|Default|GetFishGroup_02) "0,-0.025000, 0" false false)
  (Transformation|AddRelativeRotation (Variables|Default|GetFishGroup_04) "0,0.200000, 0" false false)
  (CallFunction|SunLooksatCamera)
  (CallFunction|ShouldtheDolphinJump))

(event EventBeginPlay
  (|ScaleActor
    (:Finished
      (|ScaleSun
        (:Finished
          (|ScaleHouse
            (:Finished
              (|ScaleBoat
                (:Finished
                  (|PlayAnimations)
                  (Utilities|Time|SetTimerbyEvent (delegate Custom|MoveFish) 0.01 true))))))))))

(fn ConstructionScript
  (|CallParentFunction)
  (Transformation|SetWorldRotation (Variables|Default|GetSun_Shine_Point8) "0, 0, 0" false false)
  (Rendering|SetActorHiddenInGame true)
  ;[1 1 1] Hide all skeletal meshes in game
  (for _array_element (Actor|GetComponentsbyTag "/Script/Engine.SkeletalMeshComponent" "Play")
    (Development|SetHiddeninGame _array_element true false)
    (Variables|/Script/Engine.SkeletalMeshComponent|SetbPauseAnims _array_element true)))

(fn ShouldtheDolphinJump
  (bind _asdolphin_root_skeleton_anim_blueprint (Utilities|Casting|CastToDolphin_Root_Skeleton_AnimBlueprint (Components|SkeletalMesh|GetAnimInstance (Variables|Default|GetDolphin_01))))
  (Variables|/Game/Custom/Meshes/Dolphin/Dolphin_Root_Skeleton_AnimBlueprint.Dolphin_Root_Skeleton_AnimBlueprint_C|SetJump _asdolphin_root_skeleton_anim_blueprint (< (Math|Float|Absolute(Float) (Math|Vector|VectorLength (- (Transformation|GetWorldLocation (Variables|Default|GetBoat)) (Transformation|GetWorldLocation (Variables|Default|GetDolphin_01))))) 2e+01)))

(fn SunLooksatCamera
  (Transformation|SetWorldRotation (Variables|Default|GetSun_Shine_Point8) (Math|Rotator|FindLookatRotation (Transformation|GetWorldLocation (Variables|Default|GetSun_Shine_Point8)) (Camera|GetCameraLocation (Game|GetPlayerCameraManager 0))) false false))